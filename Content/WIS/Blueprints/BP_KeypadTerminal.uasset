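; BP_KeypadTerminal is a keypad terminal that sets connected systems to an activated or deactivated state when the correct code is submitted.
; Its code is either randomly generated at BeginPlay or numeric-checked in the construction script, then passed to WBP_KeypadTerminal, whose dispatchers report submissions.
; It also listens to the first connected system, disabling the keypad when that system reaches the target state and reactivating it otherwise.
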(event EventBeginPlay
  ;[0 0.7379 1] Begin Play: Bind functions to widget events and set code
  (if (Variables|KeypadSettings|GetRandomCode?)
    (Utility|GenerateRandomCode))
  (Initialize|InitializeKeypadWidget)
  (Systems|BindSystemNotifyFunctions))

(fn ConstructionScript
  (|CallParentFunction)
  (if (Variables|KeypadSettings|GetRandomCode?)
    (Variables|KeypadSettings|SetCode "<RANDOM CODE>")
    (else
      (Utility|VerifyCode))))

(fn IncorrectCodeSubmitted)

(fn CorrectCodeSubmitted
  (Systems|ActivateConnectedSystems))

(fn InitializeKeypadWidget
  ;[0 0.7379 1] Bind functions to event dispatchers in keypad widget to inform this blueprint about code submission (correct / incorrect codes)
  (bind _aswbp_keypad_terminal (Utilities|Casting|CastToWBP_KeypadTerminal (UserInterface|GetWidget (Variables|Default|GetWidget))))
  (bind _output_get (Variables|RuntimeVariables|SetWidgetReference _aswbp_keypad_terminal))
  (EventDispatchers|BindEventtoOnCodeCorrect _output_get (EventDispatchers|CreateEvent :!event CorrectCodeSubmitted))
  (EventDispatchers|BindEventtoOnCodeIncorrect _output_get (EventDispatchers|CreateEvent :!event IncorrectCodeSubmitted))
  (Default|SetTargetCode _output_get (Variables|KeypadSettings|GetCode)))

(fn VerifyCode
  (if (not (Class|KismetStringLibrary|IsNumeric (Variables|KeypadSettings|GetCode)))
    (Variables|KeypadSettings|SetCode "TARGET CODE MUST BE NUMERIC!")))

(fn ActivateConnectedSystems
  (bind _outcomponents (CallFunction|GetConnectedSystems (Variables|KeypadSettings|GetConnectedSystemIDs)))
  (for _array_element _outcomponents
    (bind _active (Class|BPIWISFunctionInterface|SystemGetState(Message) _array_element))
    (if (Math|Boolean|NotEqual(Boolean) _active (Variables|KeypadSettings|GetShouldActivate?))
      (Class|BPIWISFunctionInterface|SystemToggleState(Message) _array_element))))

(fn GenerateRandomCode
  (Variables|KeypadSettings|SetCode "")
  (for _index (range 1 (Variables|KeypadSettings|GetRandomCodeLength))
    (Variables|KeypadSettings|SetCode (Utilities|String|Append (Variables|KeypadSettings|GetCode) (Utilities|String|ToString(Integer) (Math|Random|RandomIntegerinRange 0 9))))))

(fn BindSystemNotifyFunctions
  ;[0 0.7379 1] Inform the terminal about changes of the connected system
  (bind _outcomponents (CallFunction|GetConnectedSystems (Variables|KeypadSettings|GetConnectedSystemIDs)))
  (Utilities|IsValid (Utilities|Array|Get(acopy) _outcomponents)
    (:Is%20Valid
      (EventDispatchers|BindEventtoSystemActivated (Utilities|Array|Get(acopy) _outcomponents) (EventDispatchers|CreateEvent :!event ConnectedSystemActivated))
      (EventDispatchers|BindEventtoSystemDeactivated (Utilities|Array|Get(acopy) _outcomponents) (EventDispatchers|CreateEvent :!event ConnectedSystemDeactivated)))))

(fn ConnectedSystemActivated
  (if (Variables|KeypadSettings|GetShouldActivate?)
    (bind _widgetreference (Variables|RuntimeVariables|GetWidgetReference)
      (:then
        (Default|DeactivateKeypad _widgetreference)
        (CallFunction|DisableTerminal))
      (:else))
    (else
      (bind _widgetreference_2 (Variables|RuntimeVariables|GetWidgetReference)
        (:then
          (Default|ActivateKeypad _widgetreference_2))
        (:else)))))

(fn ConnectedSystemDeactivated
  (if (Variables|KeypadSettings|GetShouldActivate?)
    (bind _widgetreference (Variables|RuntimeVariables|GetWidgetReference)
      (:then
        (Default|ActivateKeypad _widgetreference))
      (:else))
    (else
      (bind _widgetreference_2 (Variables|RuntimeVariables|GetWidgetReference)
        (:then
          (Default|DeactivateKeypad _widgetreference_2)
          (CallFunction|DisableTerminal))
        (:else)))))