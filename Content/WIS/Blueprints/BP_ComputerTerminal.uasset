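; BP_ComputerTerminal is an in-world computer terminal that displays data from a data table row on a widget component.
; On BeginPlay it validates the widget, casts it to WBP_ComputerTerminal and caches the reference.
; It then looks up the row named by its DataRow handle and, if found, passes it to the widget through UpdateTerminalData.
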(event EventBeginPlay
  ;[0 0.7379 1] Begin Play: Set widget data
  (|CallParentFunction)
  (if (CallFunction|WidgetValid?)
    (CallFunction|PrepareTerminalWidget)))

(fn ConstructionScript
  (|CallParentFunction))

(fn PrepareTerminalWidget
  (bind _datarow (Variables|Settings|GetDataRow))
  (bind (_datatable _rowname) (Utilities|Struct|BreakDataTableRowHandle _datarow))
  ;[0 0.7379 1] Read data from table and pass it to the widget component's terminal widget
  (bind _aswbp_computer_terminal (Utilities|Casting|CastToWBP_ComputerTerminal (UserInterface|GetWidget (Variables|Default|GetWidget))))
  (bind _output_get (Variables|Default|SetTerminalWidget _aswbp_computer_terminal))
  (bind _returnvalue (Utilities|GetDataTableRow _datatable _rowname)
    (:then
      (Default|UpdateTerminalData _output_get _returnvalue))))