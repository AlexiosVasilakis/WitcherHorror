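; Base actor for an in-world terminal that zooms the view onto a 3D widget and hands player input to it.
; Focus starts from an Interact message or, with auto-focus, a timer-driven dwell trace inside the proximity trigger.
; Look input rotates a gimbal-mounted WidgetInteraction, whose hit point drives the widget's cursor.
; Movement, E in manual mode, or aiming past the border tolerance for a delay returns control to the pawn.
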(event OnComponentBeginOverlap(InteractionTrigger)
  (params (OverlappedComponent :type Primitive%20Component%20Object%20Reference) (OtherActor :type Actor%20Object%20Reference) (OtherComp :type Primitive%20Component%20Object%20Reference) (OtherBodyIndex :type Integer) (bFromSweep :type Boolean) (SweepResult :type Hit%20Result%20Structure%20%28by%20ref%29))
  ;[0 0.7379 1] Proximity trigger: Trace for interaction only in range of terminal
  (if (== OtherActor (Game|Player|GetPlayerPawn 0))
    (Activation|AllowInteraction)))

(event OnComponentEndOverlap(InteractionTrigger)
  (params (OverlappedComponent :type Primitive%20Component%20Object%20Reference) (OtherActor :type Actor%20Object%20Reference) (OtherComp :type Primitive%20Component%20Object%20Reference) (OtherBodyIndex :type Integer))
  ;[0 0.7379 1] Proximity trigger: Trace for interaction only in range of terminal
  (if (== OtherActor (Game|Player|GetPlayerPawn 0))
    (Activation|DisableInteraction false)))

(event EventInteract
  ;[1 0.4969 0] Example interaction system implementation - You might want to remove or modify this!
  ;;[1 1 1] Manual interaction with terminal: Start interaction on interface message (Interact)
  (if (not (Variables|Settings|GetAutoFocusOnTerminal))
    (switch Utilities|FlowControl|Switch|SwitchonEWidgetInteractionStates (Variables|Interaction|GetInteractionState)
      (:NewEnumerator3
        (Interaction|StartInteraction false)))))

(event EventActorFocusStart
  ;[1 0.4969 0] Example interaction system implementation - You might want to remove or modify this!
  ;;[1 1 1] Show / hide interaction prompt
  (if (not (Variables|Settings|GetAutoFocusOnTerminal))
    (Rendering|SetVisibility (Variables|Default|GetInteractionPrompt) true false)))

(event EventActorFocusEnd
  ;[1 0.4969 0] Example interaction system implementation - You might want to remove or modify this!
  ;;[1 1 1] Show / hide interaction prompt
  (if (not (Variables|Settings|GetAutoFocusOnTerminal))
    (Rendering|SetVisibility (Variables|Default|GetInteractionPrompt) false false)))

(event EventBeginPlay
  ;[0 0.7379 1] Update collision on interaction trigger (won't always update properly on construction)
  (Collision|SetCollisionEnabled (Variables|Default|GetInteractionTrigger) (select (Variables|Settings|GetAutoFocusOnTerminal) "QueryOnly" "NoCollision")))

(event Input|AxisEvents|InputAxisTurn
  (params (AxisValue :type Float%20%28single-precision%29))
  ;[0 0.7379 1] General input processing
  (Transformation|AddLocalRotation (Variables|Default|GetZ_Gimbal) (Math|Rotator|MakeRotator 0.0 0.0 (* AxisValue (Variables|Input|GetXSensitivity))) false false))

(event Input|AxisEvents|InputAxisLookUp
  (params (AxisValue :type Float%20%28single-precision%29))
  ;[0 0.7379 1] General input processing
  (Transformation|AddLocalRotation (Variables|Default|GetWidgetInteraction) (Math|Rotator|MakeRotator 0.0 (* AxisValue (Variables|Input|GetYSensitivity) -1.0) 0.0) false false))

(event Input|AxisEvents|InputAxisMoveForward
  (params (AxisValue :type Float%20%28single-precision%29))
  ;[0 0.7379 1] General input processing
  (if (Math|Float|NearlyEqual(Float) AxisValue -1.0 0.01)
    (Interaction|EndInteraction)))

(event Input|AxisEvents|InputAxisMoveRight
  (params (AxisValue :type Float%20%28single-precision%29))
  ;[0 0.7379 1] General input processing
  (if (Math|Float|NearlyEqual(Float) (Math|Float|Absolute(Float) AxisValue) 1.0 0.01)
    (Interaction|EndInteraction)))

(event Input|MouseEvents|MouseWheelAxis
  (params (AxisValue :type Float%20%28single-precision%29))
  ;[0 0.7379 1] Widget interaction input
  (Class|WidgetInteractionComponent|ScrollWheel (Variables|Default|GetWidgetInteraction) AxisValue)
  (Class|WidgetBlueprintLibrary|SetFocustoGameViewport) ; prevent locking on widget (UE5)
)

(event Input|MouseEvents|LeftMouseButton
  (params (Key :type Key%20Structure :default "None"))
  (bind _widgetinteraction (Variables|Default|GetWidgetInteraction))
  ;[0 0.7379 1] Widget interaction input
  (:Pressed
    (Class|WidgetInteractionComponent|PressPointerKey _widgetinteraction "LeftMouseButton")
    (Class|WidgetBlueprintLibrary|SetFocustoGameViewport :!label _label) ; prevent locking on widget (UE5)
  )
  (:Released
    (Class|WidgetInteractionComponent|ReleasePointerKey _widgetinteraction "LeftMouseButton")
    (goto _label)))

(event Input|KeyboardEvents|E
  (params (Key :type Key%20Structure :default "None"))
  ;[1 0.4969 0] Example interaction system implementation - You might want to remove or modify this!
  ;;[1 1 1] End interacction on interaction button input
  (:Pressed
    (if (not (Variables|Settings|GetAutoFocusOnTerminal))
      (switch Utilities|FlowControl|Switch|SwitchonEWidgetInteractionStates (Variables|Interaction|GetInteractionState)
        (:NewEnumerator1
          (Interaction|EndInteraction))))))

(fn ConstructionScript
  ;[0 0.7379 1] Interaction trigger setup
  (Construction|UpdateCameraSettings)
  (Components|Sphere|SetSphereRadius (Variables|Default|GetInteractionTrigger) (Variables|Settings|GetTraceDistance) true)
  (Transformation|SetRelativeLocation (Variables|Default|GetInteractionTrigger) (Math|Vector|MakeVector (* (Variables|Settings|GetTraceDistance) -1.0) 0.0 0.0) false false))

(fn TraceforInteraction
  (bind _returnvalue (Game|GetPlayerCameraManager 0))
  (bind _returnvalue_2 (Camera|GetCameraLocation _returnvalue))
  (if (Math|Float|NearlyEqual(Float) (Math|Vector|VectorLength (Transformation|GetVelocity (Game|Player|GetPlayerPawn 0))) 0.0 1.0)
    (bind _outhit (Collision|LineTraceByChannel _returnvalue_2 (+ _returnvalue_2 (* (Transformation|GetActorForwardVector _returnvalue) (Variables|Settings|GetTraceDistance))) "TraceTypeQuery1" false 0 "None" false))
    (if (.bblockinghit _outhit)
      (Variables|Activation|SetInitialHitLocation (.impactpoint _outhit))
      (if (== (Variables|Default|GetWidget) (.hitcomponent _outhit))
        (bind _returnvalue_3 (Utility|HitWithinInnerArea?))
        (if _returnvalue_3
          (bind _output_get (Variables|Activation|SetCurrentDetectActivationTime (+ (Variables|Activation|GetCurrentDetectActivationTime) (Utilities|Time|GetWorldDeltaSeconds))))
          (if (> _output_get (Variables|Settings|GetActivationDetectionDuration))
            (Variables|Activation|SetCurrentDetectActivationTime 0.0)
            (Utilities|Time|ClearandInvalidateTimerbyHandle (Variables|Timers|GetTraceForFocusTimer))
            (Interaction|StartInteraction true))
          (else
            (Variables|Activation|SetCurrentDetectActivationTime 0.0 :!label _label)))
        (else
          (goto _label)))
      (else
        (goto _label)))
    (else
      (Variables|Activation|SetCurrentDetectActivationTime 0.0))))

(fn StartInteraction
  (params (UseInitialHit :type Boolean))
  (bind (_valid _interactioncomponent) (CallFunction|GetInteractionComponent))
  (bind _returnvalue (Game|GetPlayerController 0))
  (bind _widgetinteraction (Variables|Default|GetWidgetInteraction))
  (Variables|Interaction|SetInteractionState "NewEnumerator0")
  (Utilities|Time|ClearandInvalidateTimerbyHandle (Variables|Timers|GetEndInteractionTimer))
  (Utilities|FlowControl|Sequence
    (:then_0
      ;[1 0.4969 0] You might want to remove this, if you're not using this asset's example interaction system!
      (if _valid
        (Default|PauseInteraction _interactioncomponent)))
    (:then_1
      ;[0 0.7379 1] Change input permissions
      (Input|DisableInput (Game|Player|GetPlayerPawn 0) _returnvalue)
      (Input|EnableInput _returnvalue)
      ;[0 0.7379 1] Smoothly change active camera
      (Game|Player|SetViewTargetwithBlend (Game|GetPlayerController 0) self (Variables|Settings|GetZoomInDuration) "VTBlend_Cubic" 0.0 false)
      (if UseInitialHit
        ;[0 0.7379 1] Set initial rotation for widget interaction to match hit location on screen
        (Transformation|SetRelativeRotation (Variables|Default|GetWidgetInteraction) (Math|Transform|InverseTransformRotation (Transformation|GetWorldTransform _widgetinteraction) (Math|Rotator|FindLookatRotation (Transformation|GetWorldLocation _widgetinteraction) (Variables|Activation|GetInitialHitLocation))) false false)
        ;[0 0.7379 1] Show cursor at initial location
        (Class|BPIWISFunctionInterface|ShowCursor(Message) (UserInterface|GetWidget (Variables|Default|GetWidget)) (Utility|TransformWorldtoWidgetLocation (Variables|Activation|GetInitialHitLocation)))
        (else
          ;[0 0.7379 1] For interaction without auto focus: Always use origin rotation and position on interaction start
          (Transformation|SetRelativeRotation (Variables|Default|GetWidgetInteraction) "0, 0, 0" false false)
          (Class|BPIWISFunctionInterface|ShowCursor(Message) (UserInterface|GetWidget (Variables|Default|GetWidget)))))
      ;[0 0.7379 1] Enable interaction with 3D widget
      (Components|Activation|Activate (Variables|Default|GetWidgetInteraction) false)
      ;[0 0.7379 1] Execute required events on timers (cursor updates / cooldowns)
      (bind _returnvalue_2 (Utilities|Time|SetTimerbyEvent (EventDispatchers|CreateEvent :!event UpdateCursorandDetectOutOfScreen) (Utilities|Time|GetWorldDeltaSeconds) true))
      (Variables|Timers|SetCursorUpdateTimer _returnvalue_2)
      (Utilities|Time|SetTimerbyEvent (EventDispatchers|CreateEvent :!event UpdatePlayerLocation) (Variables|Settings|GetZoomInDuration)) ; When in full focus, update player's location to match camera location
      (Utilities|Time|SetTimerbyEvent (EventDispatchers|CreateEvent :!event HandleInteractionCooldown) (Variables|Interaction|GetInteractionCooldownTime))
      (Variables|Interaction|SetInteractionState "NewEnumerator1"))))

(fn EndInteraction
  (bind (_valid _interactioncomponent) (CallFunction|GetInteractionComponent))
  (bind _returnvalue (Game|GetPlayerController 0))
  (bind _widgetinteraction (Variables|Default|GetWidgetInteraction))
  (bind _returnvalue_2 (Transformation|GetWorldRotation _widgetinteraction))
  (Variables|Interaction|SetInteractionState "NewEnumerator2")
  (if (Components|Activation|IsActive (Variables|Default|GetWidgetInteraction))
    (Class|BPIWISFunctionInterface|HideCursor(Message) (UserInterface|GetWidget (Variables|Default|GetWidget)))
    (Components|Activation|Deactivate (Variables|Default|GetWidgetInteraction))
    (Pawn|SetControlRotation (Game|GetPlayerController 0) (Math|Rotator|MakeRotator 0.0 (.pitch _returnvalue_2) (.yaw _returnvalue_2)))
    (Utilities|Time|ClearandInvalidateTimerbyHandle (Variables|Timers|GetCursorUpdateTimer))
    (Input|DisableInput _returnvalue)
    (Input|EnableInput (Game|Player|GetPlayerPawn 0) _returnvalue)
    (Game|Player|SetViewTargetwithBlend (Game|GetPlayerController 0) (Game|Player|GetPlayerPawn 0) 0.3 "VTBlend_Cubic" 0.0 false)
    (Utilities|Time|SetTimerbyEvent (EventDispatchers|CreateEvent :!event ReenableInteraction) 1.0)
    ;[1 0.4934 0] You might want to remove this, if you're not using this asset's example interaction system!
    (if _valid
      (Default|ResumeInteraction _interactioncomponent))))

(fn ReenableInteraction
  (if (Utilities|Enum|Equal(Enum) (Variables|Interaction|GetInteractionState) "NewEnumerator2")
    (Transformation|SetRelativeRotation (Variables|Default|GetWidgetInteraction) "0, 0, 0" false false)
    (Variables|Interaction|SetInteractionState "NewEnumerator3")
    (if (Variables|Settings|GetAutoFocusOnTerminal)
      (bind _returnvalue (Utilities|Time|SetTimerbyEvent (EventDispatchers|CreateEvent :!event TraceforInteraction) (Utilities|Time|GetWorldDeltaSeconds) true))
      (Variables|Timers|SetTraceForFocusTimer _returnvalue))))

(fn EndInteractionwithDelay
  (if (not (Utilities|Time|IsTimerActivebyHandle (Variables|Timers|GetEndInteractionTimer)))
    (bind _returnvalue (Utilities|Time|SetTimerbyEvent (EventDispatchers|CreateEvent :!event EndInteraction) (Variables|Settings|GetEndInteractionDelay)))
    (Variables|Timers|SetEndInteractionTimer _returnvalue)))

(fn UpdateCursorandDetectOutOfScreen
  (bind _widgetinteraction (Variables|Default|GetWidgetInteraction))
  (bind _returnvalue (Class|WidgetInteractionComponent|GetLastHitResult _widgetinteraction))
  (if (.bblockinghit _returnvalue)
    (Utilities|Time|ClearandInvalidateTimerbyHandle (Variables|Timers|GetEndInteractionTimer))
    (if (== (Variables|Default|GetWidget) (.hitcomponent _returnvalue))
      (Class|BPIWISFunctionInterface|UpdateCursorPosition(Message) (UserInterface|GetWidget (Variables|Default|GetWidget)) (Utility|TransformWorldtoWidgetLocation (.impactpoint _returnvalue)))
      (else
        (bind _returnvalue_2 (Utility|IsHitinTolerance? :!label _label))
        (if _returnvalue_2
          (Utilities|Time|ClearandInvalidateTimerbyHandle (Variables|Timers|GetEndInteractionTimer))
          (else
            (Interaction|EndInteractionwithDelay)))))
    (else
      (goto _label))))

(fn UpdatePlayerLocation
  (bind _widget (Variables|Default|GetWidget))
  (bind _returnvalue (Transformation|GetWorldLocation _widget))
  (Transformation|SetActorLocation (Game|Player|GetPlayerPawn 0) (+ (* (Class|KismetMathLibrary|VectorNormal2D (Math|Vector|GetUnitDirection(Vector) (Transformation|GetWorldLocation (Variables|Default|GetWidget)) (Transformation|GetWorldLocation (Variables|Default|GetCamera))) 0.0001) (Variables|Settings|GetRepositionOffset)) (Math|Vector|MakeVector (.x _returnvalue) (.y _returnvalue) (.z (Transformation|GetActorLocation (Game|Player|GetPlayerPawn 0))))) false false))

(fn HitWithinInnerArea?
  (bind _returnvalue (Game|GetPlayerCameraManager 0))
  (bind _returnvalue_2 (Camera|GetCameraLocation _returnvalue))
  (Collision|SetCollisionEnabled (Variables|Default|GetInnerWidgetArea) "QueryOnly")
  (bind _outhit (Collision|LineTraceByChannel _returnvalue_2 (+ _returnvalue_2 (* (Transformation|GetActorForwardVector _returnvalue) (Variables|Settings|GetTraceDistance))) "TraceTypeQuery1" false 0 "None" false))
  (if (.bblockinghit _outhit)
    (if (== (Variables|Default|GetInnerWidgetArea) (.hitcomponent _outhit))
      (Collision|SetCollisionEnabled (Variables|Default|GetInnerWidgetArea) "NoCollision")
      (return true)
      (else
        (Collision|SetCollisionEnabled (Variables|Default|GetInnerWidgetArea) "NoCollision")
        (return false)))
    (else
      (Collision|SetCollisionEnabled (Variables|Default|GetInnerWidgetArea) "NoCollision")
      (return false))))

(fn IsHitinTolerance?
  (bind _widgetinteraction (Variables|Default|GetWidgetInteraction))
  (bind _returnvalue (Transformation|GetWorldLocation _widgetinteraction))
  (bind (_outhits _returnvalue_2) (Collision|MultiSphereTraceByChannel _returnvalue (+ _returnvalue (* (Math|Vector|GetForwardVector _widgetinteraction) (Variables|Settings|GetTraceDistance))) (Variables|Settings|GetWidgetBorderHitTolerance) "TraceTypeQuery1" true 0 "None" false))
  (if _returnvalue_2
    (bind _array_element (Utilities|Array|ForEachLoopwithBreak _outhits :!label _label)
      (:LoopBody
        (if (== (Variables|Default|GetWidget) (.hitcomponent _array_element))
          (LocalVariables|SetWidgetInRange true)
          (goto _label Break)))
      (:Completed
        (return (LocalVariables|GetWidgetInRange))))
    (else
      (return false))))

(fn TransformWorldtoWidgetLocation
  (params (InputPin :type Vector))
  (bind _widget (Variables|Default|GetWidget))
  (bind _returnvalue (Transformation|GetWorldTransform _widget))
  (bind _returnvalue_2 (Math|Transform|InverseTransformLocation _returnvalue InputPin))
  (return (Class|KismetMathLibrary|Negated2D (Math|Vector2D|MakeVector2D (.y _returnvalue_2) (.z _returnvalue_2)))))

(fn AllowInteraction
  (if (Utilities|Enum|Equal(Enum) (Variables|Interaction|GetInteractionState) "NewEnumerator3")
    (if (Variables|Settings|GetAutoFocusOnTerminal)
      (bind _returnvalue (Utilities|Time|SetTimerbyEvent (EventDispatchers|CreateEvent :!event TraceforInteraction) (Utilities|Time|GetWorldDeltaSeconds) true))
      (Variables|Timers|SetTraceForFocusTimer _returnvalue))))

(fn DisableInteraction
  (params (Force :type Boolean))
  (if (or (Utilities|Enum|Equal(Enum) (Variables|Interaction|GetInteractionState) "NewEnumerator1") Force)
    (Utilities|Time|ClearandInvalidateTimerbyHandle (Variables|Timers|GetTraceForFocusTimer))))

(fn HandleInteractionCooldown
  (Variables|Interaction|SetAllowInteractionEnd true))

(fn WidgetValid?
  (bind _widget (Variables|Default|GetWidget)
    (:then
      (Utilities|IsValid (UserInterface|GetWidget _widget)
        (:Is%20Valid
          (return true))
        (:Is%20Not%20Valid
          _)))
    (:else
      _))
  (return false))

(fn UpdateCameraSettings
  ;[0 0.7379 1] Calculate and apply focal distance and auto exposure values
  (Utilities|Struct|SetmembersinPostProcessSettings (Variables|/Script/Engine.CameraComponent|GetPostProcessSettings (Variables|Default|GetCamera)) (Variables|Settings|GetCameraAutoExposureLowPercent) (Math|Vector|Distance(Vector) (Transformation|GetWorldLocation (Variables|Default|GetCamera)) (Transformation|GetWorldLocation (Variables|Default|GetWidget)))))

(fn DisableTerminal
  (Variables|Interaction|SetInteractionState "NewEnumerator4")
  (Collision|SetCollisionEnabled (Variables|Default|GetInteractionTrigger) "NoCollision")
  (Interaction|EndInteraction)
  (Activation|DisableInteraction true))

(fn EnableTerminal
  (Collision|SetCollisionEnabled (Variables|Default|GetInteractionTrigger) "QueryOnly")
  (Variables|Interaction|SetInteractionState "NewEnumerator3"))