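; Switch terminal with a widget button that toggles systems linked by ID and displays their on/off state.
; On Begin Play it sets the widget title, binds the button event, resolves connected systems and subscribes to their activated/deactivated dispatchers.
; Toggling only flips systems matching the terminal's current state, keeping mixed groups from inverting.
; System reports update that state and the button text, so the label follows the systems rather than the press.
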(event EventBeginPlay
  ;[0 0.7379 1] Begin Play: Prepare connected system(s) and bind functions to widget events
  (Initialize|InitializeSwitchWidget)
  (Initialize|InitializeSystems))

(fn ConstructionScript
  (|CallParentFunction))

(fn InitializeSwitchWidget
  ;[0 0.7379 1] Bind functions to event dispatchers in widget to inform this blueprint about button events.
  (bind _aswbp_simple_switch_terminal (Utilities|Casting|CastToWBP_SimpleSwitchTerminal (UserInterface|GetWidget (Variables|Default|GetWidget))))
  (bind _output_get (Variables|RuntimeVariable|SetSwitchTerminalWidget _aswbp_simple_switch_terminal))
  (EventDispatchers|BindEventtoButtonPressed _output_get (EventDispatchers|CreateEvent :!event ToggleConnectedSystems))
  (Default|UpdateTitleText _output_get (Variables|Settings|GetTitleText)))

(fn ToggleConnectedSystems
  (bind _outcomponents (CallFunction|GetConnectedSystems (Variables|Settings|GetConnectedSystemIDs)))
  (for _array_element _outcomponents
    (bind _active (Class|BPIWISFunctionInterface|SystemGetState(Message) _array_element))
    (if (Math|Boolean|Equal(Boolean) _active (Variables|RuntimeVariable|GetSystemState))
      (Class|BPIWISFunctionInterface|SystemToggleState(Message) _array_element))))

(fn InitializeSystems
  (bind _outcomponents (CallFunction|GetConnectedSystems (Variables|Settings|GetConnectedSystemIDs)))
  (bind _output_get (Variables|RuntimeVariable|SetConnectedSystems _outcomponents))
  (for _array_element _output_get
    (EventDispatchers|BindEventtoSystemActivated _array_element (EventDispatchers|CreateEvent :!event SystemReportsActivated))
    (EventDispatchers|BindEventtoSystemDeactivated _array_element (EventDispatchers|CreateEvent :!event SystemReportsDeactivated)))
  (Variables|RuntimeVariable|SetSystemState (CallFunction|GetConnectedSystemsState (Variables|RuntimeVariable|GetConnectedSystems)))
  (CallFunction|UpdateButtonText))

(fn SystemReportsDeactivated
  (Variables|RuntimeVariable|SetSystemState false)
  (CallFunction|UpdateButtonText))

(fn SystemReportsActivated
  (Variables|RuntimeVariable|SetSystemState true)
  (CallFunction|UpdateButtonText))

(fn UpdateButtonText
  (Default|UpdateButtonText (Variables|RuntimeVariable|GetSwitchTerminalWidget) (select (Variables|RuntimeVariable|GetSystemState) (Variables|Settings|GetButtonTextActive) (Variables|Settings|GetButtonTextInactive))))