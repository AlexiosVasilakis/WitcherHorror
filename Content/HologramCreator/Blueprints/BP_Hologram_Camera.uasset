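; Scene capture camera actor for holograms that renders to an assigned render target and carries a rotating movement component with a configurable rate.
; Construction and BeginPlay apply the render target and rotation rate.
; A debug-drawn line trace along the capture's pitch measures height above ground and sends it to referenced Niagara hologram systems.
; This measurement runs at construction and every tick only when enabled; otherwise tick disables itself.
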(event EventBeginPlay
  (CallFunction|WrapperSetters))

(event EventTick
  (params (DeltaSeconds :type Float%20%28single-precision%29))
  ;[0.4886 1 0.7156] Disable tick unless it is required for updating the distance in real time.
  (if (Variables|HologramCreator|GetUpdate%20Distance%20on%20Tick)
    (CallFunction|CalculateandSaveDistance)
    (else
      (Actor|Tick|SetActorTickEnabled false))))

(fn ConstructionScript
  (CallFunction|WrapperSetters)
  (if (Variables|HologramCreator|GetUpdate%20Distance%20on%20Tick)
    (CallFunction|CalculateandSaveDistance)))

(fn CalculateandSaveDistance
  (bind _scenecapturecomponent2d (Variables|Default|GetSceneCaptureComponent2D))
  (bind _returnvalue (Transformation|GetWorldLocation _scenecapturecomponent2d))
  ;[0.3491 1 0.4555] Perform line trace in "forward" direction of the SceneCaptureComponent. Since the SceneCaptureComp is facing down, this trace will be straight down and will calculate the distance to the floor. I.e. it will determine the height of this actor.
  (bind _outhit (Collision|LineTraceByChannel _returnvalue (+ _returnvalue (* (Math|Vector|GetForwardVector (Math|Rotator|MakeRotator 0.0 (.Pitch (Math|Rotator|BreakRotator (Transformation|GetWorldRotation _scenecapturecomponent2d))) 0.0)) 1e+07)) "TraceTypeQuery1" false 0 "ForDuration" true "(R=1.000000,G=0.000000,B=0.000000,A=1.000000)" "(R=0.000000,G=1.000000,B=0.000000,A=1.000000)" 0.05))
  ;[0.284 0.9002 1] Save the distance.
  (bind _output_get (Variables|Default|SetHeight%20Above%20Ground (.Distance (Collision|BreakHitResult _outhit))))
  ;[0.9273 1 0.5086] Update all referenced hologram systems with the current height.
  (for _array_element (Variables|HologramCreator|GetHologramParticleSystems)
    (Effects|Components|ParticleSystem|SetFloatParameter (Variables|/Script/Niagara.NiagaraActor|GetNiagaraComponent _array_element) "Camera Height Above Ground" _output_get)))

(fn WrapperSetters
  (Variables|/Script/Engine.SceneCaptureComponent2D|SetTextureTarget (Variables|Default|GetSceneCaptureComponent2D) (Variables|HologramCreator|GetRender%20Target))
  (Variables|/Script/Engine.RotatingMovementComponent|SetRotationRate (Variables|Default|GetRotatingMovement) (Math|Rotator|MakeRotator 0.0 0.0 (Variables|HologramCreator|GetRotation%20Rate))))